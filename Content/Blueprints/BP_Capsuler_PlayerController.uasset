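; Player controller for the Capsuler pawn that handles forward/backward movement and jumping.
; BeginPlay caches player 0's pawn and character, and Tick stores delta time for the movement input.
; The MoveForward axis is eased with FInterpTo, scaled by Speed and applied along the yaw-only control rotation.
; Jump press triggers the character's jump, while release only prints a debug string.
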(event EventBeginPlay
  (Variables|Default|SetTCPawn (Game|Player|GetPlayerPawn 0))
  (Variables|Default|SetTCCharacter (Game|GetPlayerCharacter 0)))

(event EventTick
  (params (DeltaSeconds :type Float%20%28single-precision%29))
  (Variables|Default|SetDelta DeltaSeconds))

(event Input|ActionEvents|InputActionJump
  (params (Key :type Key%20Structure))
  (:Pressed
    (Development|PrintString "Jump")
    (Character|Jump (Variables|Default|GetTCCharacter)))
  (:Released
    (Development|PrintString "Release")))

(event Input|AxisEvents|InputAxisMoveForward
  (params (AxisValue :type Float%20%28single-precision%29))
  (bind _output_get (Variables|Default|SetCurrentForwardValue (Math|Interpolation|FInterpTo (Variables|Default|GetCurrentForwardValue) AxisValue (Variables|Default|GetDelta) 5.0)))
  (Pawn|Input|AddMovementInput (Variables|Default|GetTCPawn) (Math|Vector|GetForwardVector (Math|Rotator|MakeRotator 0.0 0.0 (.Yaw (Math|Rotator|BreakRotator (Pawn|GetControlRotation (Variables|Default|GetTCPawn) :!class /Script/Engine.Pawn))))) (* _output_get (Variables|Default|GetSpeed)) false))

(fn ConstructionScript)